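; Configurable light rig actor that builds a set of point, spot and rect lights around itself from the LightingSetup array.
; The construction script unpacks each entry through LightData, then adds a spring arm with its length and rotation to position the light.
; A light of the chosen type is attached to that arm and receives the shared and type-specific settings.
; ApplyPreSet replaces LightingSetup with the entries from a RigPreset.
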(fn `ApplyPreSet`
  (`KismetArrayLibrary.Array_Clear` (`self.Lighting Setup`))
  (bind _rigpreset (`self.RigPreset`)
    (:`then`
      (for _array_element (`/Game/Light/presets/DA_LightRigPreset.PRESETLightSetup` _rigpreset)
        (`KismetArrayLibrary.Array_Add` (`self.Lighting Setup`) _array_element)))
    (:`else`)))

(fn `LightData`
  (params (S_LightingData :type "/Game/Light/Bluepint/Light/S_LightingData Structure (by ref)"))
  (returns (PointLightSetting :type "/Game/Light/Bluepint/Light/S_PointLightSetting Structure") (OutputPin :type "Float (double-precision)") (SpotLightSetting :type "/Game/Light/Bluepint/Light/S_SpotLightSetting Structure") (RectLightSetting :type "/Game/Light/Bluepint/Light/S_RectLightSetting Structure"))
  (bind (_armlength _armrota _lightingintensity _lightingcolor _lightingtem _lighttype _attenuationradius _rectlightsetting _spotlightsetting _pointlightsetting) (break `/Game/Light/Bluepint/Light/S_LightingData` S_LightingData))
  (set `self.Arm Length` _armlength)
  (set `self.Arm ROTA` _armrota)
  (set `self.Lighting Color` _lightingcolor)
  (set `self.Lighting Tem` _lightingtem)
  (set `self.Light Type` _lighttype)
  (set `self.Attenuation Radius` _attenuationradius)
  (return _pointlightsetting _lightingintensity _spotlightsetting _rectlightsetting))

(fn `Spring  Arm Setting`
  (params (InputPin :type "Float (double-precision)"))
  (bind _returnvalue (`AddComponent|NODE_AddSpringArmComponent-0`))
  (set `self.Spring Arm` _returnvalue)
  (set `SpringArmComponent.TargetArmLength` (`self.Arm Length`) (`self.Spring Arm`))
  (`SceneComponent.K2_AddRelativeRotation` (`self.Spring Arm`) (`self.Arm ROTA`) false false)
  (set `self.Lighting Intensity` InputPin))

(fn `UserConstructionScript`
  (bind _rect_light (`self.Rect Light`))
  (bind _spot_light (`self.Spot Light`))
  (bind _point_light (`self.Point Light`))
  (for _array_element (`self.Lighting Setup`)
    (bind (_pointlightsetting _outputpin _spotlightsetting _rectlightsetting) (`self.LightData` _array_element))
    ; Spring  Arm Setting
    (`self.Spring  Arm Setting` _outputpin)
    (switch `/Game/Light/Bluepint/Light/E_LightType` (`self.Light Type`)
      (:`NewEnumerator0`
        ; Create Point Light Setting
        (bind _returnvalue (`AddComponent|NODE_AddPointLightComponent-0`))
        (set `self.Point Light` _returnvalue)
        (`SceneComponent.K2_AttachToComponent` (`self.Point Light`) (`self.Spring Arm`) "None" "KeepRelative" "KeepRelative" "KeepRelative" true)
        (`LightComponent.SetIntensity` (`self.Point Light`) (`self.Lighting Intensity`))
        (`LightComponent.SetLightColor` (`self.Point Light`) (`KismetMathLibrary.Conv_ColorToLinearColor` (`self.Lighting Color`)) true)
        (`LightComponent.SetTemperature` (`self.Point Light`) (`self.Lighting Tem`))
        (`LocalLightComponent.SetAttenuationRadius` (`self.Point Light`) (`self.Attenuation Radius`))
        (bind (_sourceradius _sourcelength) (break `/Game/Light/Bluepint/Light/S_PointLightSetting` _pointlightsetting))
        (`PointLightComponent.SetSourceRadius` _point_light _sourceradius)
        (`PointLightComponent.SetSourceLength` _point_light _sourcelength))
      (:`NewEnumerator1`
        ; Create Spot Light Setting
        (bind _returnvalue_2 (`AddComponent|NODE_AddSpotLightComponent-0`))
        (set `self.Spot Light` _returnvalue_2)
        (`SceneComponent.K2_AttachToComponent` (`self.Spot Light`) (`self.Spring Arm`) "None" "KeepRelative" "KeepRelative" "KeepRelative" true)
        (`LightComponent.SetIntensity` (`self.Spot Light`) (`self.Lighting Intensity`))
        (`LightComponent.SetLightColor` (`self.Spot Light`) (`KismetMathLibrary.Conv_ColorToLinearColor` (`self.Lighting Color`)) true)
        (`LightComponent.SetTemperature` (`self.Spot Light`) (`self.Lighting Tem`))
        (`LocalLightComponent.SetAttenuationRadius` (`self.Spot Light`) (`self.Attenuation Radius`))
        (bind (_innercone _outercone _sourceradius_2 _sourcelength_2) (break `/Game/Light/Bluepint/Light/S_SpotLightSetting` _spotlightsetting))
        (`SpotLightComponent.SetInnerConeAngle` _spot_light _innercone)
        (`SpotLightComponent.SetOuterConeAngle` _spot_light _outercone)
        (`PointLightComponent.SetSourceRadius` _spot_light _sourceradius_2)
        (`PointLightComponent.SetSourceLength` _spot_light _sourcelength_2))
      (:`NewEnumerator2`
        ; Create Rect  Light Setting
        (bind _returnvalue_3 (`AddComponent|NODE_AddRectLightComponent-0`))
        (set `self.Rect Light` _returnvalue_3)
        (`SceneComponent.K2_AttachToComponent` (`self.Rect Light`) (`self.Spring Arm`) "None" "KeepRelative" "KeepRelative" "KeepRelative" true)
        (`LightComponent.SetIntensity` (`self.Rect Light`) (`self.Lighting Intensity`))
        (`LightComponent.SetLightColor` (`self.Rect Light`) (`KismetMathLibrary.Conv_ColorToLinearColor` (`self.Lighting Color`)) true)
        (`LightComponent.SetTemperature` (`self.Rect Light`) (`self.Lighting Tem`))
        (`LocalLightComponent.SetAttenuationRadius` (`self.Rect Light`) (`self.Attenuation Radius`))
        (bind (_sourcewidth _sourceheight _doorangle _doorlength _sourcetex) (break `/Game/Light/Bluepint/Light/S_RectLightSetting` _rectlightsetting))
        (`RectLightComponent.SetSourceWidth` _rect_light _sourcewidth)
        (`RectLightComponent.SetBarnDoorAngle` _rect_light _doorangle)
        (`RectLightComponent.SetSourceHeight` _rect_light _sourceheight)
        (`RectLightComponent.SetBarnDoorLength` _rect_light _doorlength)
        (`RectLightComponent.SetSourceTexture` _rect_light _sourcetex)))))